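; Marimba instrument actor built from Child Actor components that each host a NoteBlock_BP, forming a chromatic keyboard from F2 to G5.
; The Construction Script casts each child and sets its NoteSound to the matching pitch, with 1w–3w repeating F2–A2 and Lo and Lolo using an explosion sound.
; The casts run in one chain, so a failed cast leaves all later blocks unassigned.
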(fn ConstructionScript
  (bind _asnote_block_bp (Utilities|Casting|CastToNoteBlock_BP (Variables|/Script/Engine.ChildActorComponent|GetChildActor (Variables|Components|Get1w))))
  (Variables|/Game/Blueprints/NoteBlock_BP.NoteBlock_BP_C|SetNoteSound _asnote_block_bp "/Game/Blueprints/f2.f2")
  (bind _asnote_block_bp_2 (Utilities|Casting|CastToNoteBlock_BP (Variables|/Script/Engine.ChildActorComponent|GetChildActor (Variables|Components|Get2w))))
  (Variables|/Game/Blueprints/NoteBlock_BP.NoteBlock_BP_C|SetNoteSound _asnote_block_bp_2 "/Game/Blueprints/g2.g2")
  (bind _asnote_block_bp_3 (Utilities|Casting|CastToNoteBlock_BP (Variables|/Script/Engine.ChildActorComponent|GetChildActor (Variables|Components|Get3w))))
  (Variables|/Game/Blueprints/NoteBlock_BP.NoteBlock_BP_C|SetNoteSound _asnote_block_bp_3 "/Game/Blueprints/a2.a2")
  (bind _asnote_block_bp_4 (Utilities|Casting|CastToNoteBlock_BP (Variables|/Script/Engine.ChildActorComponent|GetChildActor (Variables|Components|Getf2))))
  (Variables|/Game/Blueprints/NoteBlock_BP.NoteBlock_BP_C|SetNoteSound _asnote_block_bp_4 "/Game/Blueprints/f2.f2")
  (bind _asnote_block_bp_5 (Utilities|Casting|CastToNoteBlock_BP (Variables|/Script/Engine.ChildActorComponent|GetChildActor (Variables|Components|Getg2))))
  (Variables|/Game/Blueprints/NoteBlock_BP.NoteBlock_BP_C|SetNoteSound _asnote_block_bp_5 "/Game/Blueprints/g2.g2")
  (bind _asnote_block_bp_6 (Utilities|Casting|CastToNoteBlock_BP (Variables|/Script/Engine.ChildActorComponent|GetChildActor (Variables|Components|Geta2))))
  (Variables|/Game/Blueprints/NoteBlock_BP.NoteBlock_BP_C|SetNoteSound _asnote_block_bp_6 "/Game/Blueprints/a2.a2")
  (bind _asnote_block_bp_7 (Utilities|Casting|CastToNoteBlock_BP (Variables|/Script/Engine.ChildActorComponent|GetChildActor (Variables|Components|Getb2))))
  (Variables|/Game/Blueprints/NoteBlock_BP.NoteBlock_BP_C|SetNoteSound _asnote_block_bp_7 "/Game/Blueprints/b2.b2")
  (bind _asnote_block_bp_8 (Utilities|Casting|CastToNoteBlock_BP (Variables|/Script/Engine.ChildActorComponent|GetChildActor (Variables|Components|Getc3))))
  (Variables|/Game/Blueprints/NoteBlock_BP.NoteBlock_BP_C|SetNoteSound _asnote_block_bp_8 "/Game/Blueprints/c3.c3")
  (bind _asnote_block_bp_9 (Utilities|Casting|CastToNoteBlock_BP (Variables|/Script/Engine.ChildActorComponent|GetChildActor (Variables|Components|Getd3))))
  (Variables|/Game/Blueprints/NoteBlock_BP.NoteBlock_BP_C|SetNoteSound _asnote_block_bp_9 "/Game/Blueprints/d3.d3")
  (bind _asnote_block_bp_10 (Utilities|Casting|CastToNoteBlock_BP (Variables|/Script/Engine.ChildActorComponent|GetChildActor (Variables|Components|Gete3))))
  (Variables|/Game/Blueprints/NoteBlock_BP.NoteBlock_BP_C|SetNoteSound _asnote_block_bp_10 "/Game/Blueprints/e3.e3")
  (bind _asnote_block_bp_11 (Utilities|Casting|CastToNoteBlock_BP (Variables|/Script/Engine.ChildActorComponent|GetChildActor (Variables|Components|Getf3))))
  (Variables|/Game/Blueprints/NoteBlock_BP.NoteBlock_BP_C|SetNoteSound _asnote_block_bp_11 "/Game/Blueprints/f3.f3")
  (bind _asnote_block_bp_12 (Utilities|Casting|CastToNoteBlock_BP (Variables|/Script/Engine.ChildActorComponent|GetChildActor (Variables|Components|Getg3))))
  (Variables|/Game/Blueprints/NoteBlock_BP.NoteBlock_BP_C|SetNoteSound _asnote_block_bp_12 "/Game/Blueprints/g3.g3")
  (bind _asnote_block_bp_13 (Utilities|Casting|CastToNoteBlock_BP (Variables|/Script/Engine.ChildActorComponent|GetChildActor (Variables|Components|Geta3))))
  (Variables|/Game/Blueprints/NoteBlock_BP.NoteBlock_BP_C|SetNoteSound _asnote_block_bp_13 "/Game/Blueprints/a3.a3")
  (bind _asnote_block_bp_14 (Utilities|Casting|CastToNoteBlock_BP (Variables|/Script/Engine.ChildActorComponent|GetChildActor (Variables|Components|Getb3))))
  (Variables|/Game/Blueprints/NoteBlock_BP.NoteBlock_BP_C|SetNoteSound _asnote_block_bp_14 "/Game/Blueprints/b3.b3")
  (bind _asnote_block_bp_15 (Utilities|Casting|CastToNoteBlock_BP (Variables|/Script/Engine.ChildActorComponent|GetChildActor (Variables|Components|Getc4))))
  (Variables|/Game/Blueprints/NoteBlock_BP.NoteBlock_BP_C|SetNoteSound _asnote_block_bp_15 "/Game/Blueprints/c4.c4")
  (bind _asnote_block_bp_16 (Utilities|Casting|CastToNoteBlock_BP (Variables|/Script/Engine.ChildActorComponent|GetChildActor (Variables|Components|Getd4))))
  (Variables|/Game/Blueprints/NoteBlock_BP.NoteBlock_BP_C|SetNoteSound _asnote_block_bp_16 "/Game/Blueprints/d4.d4")
  (bind _asnote_block_bp_17 (Utilities|Casting|CastToNoteBlock_BP (Variables|/Script/Engine.ChildActorComponent|GetChildActor (Variables|Components|Gete4))))
  (Variables|/Game/Blueprints/NoteBlock_BP.NoteBlock_BP_C|SetNoteSound _asnote_block_bp_17 "/Game/Blueprints/e4.e4")
  (bind _asnote_block_bp_18 (Utilities|Casting|CastToNoteBlock_BP (Variables|/Script/Engine.ChildActorComponent|GetChildActor (Variables|Components|Getf4))))
  (Variables|/Game/Blueprints/NoteBlock_BP.NoteBlock_BP_C|SetNoteSound _asnote_block_bp_18 "/Game/Blueprints/f4.f4")
  (bind _asnote_block_bp_19 (Utilities|Casting|CastToNoteBlock_BP (Variables|/Script/Engine.ChildActorComponent|GetChildActor (Variables|Components|Getg4))))
  (Variables|/Game/Blueprints/NoteBlock_BP.NoteBlock_BP_C|SetNoteSound _asnote_block_bp_19 "/Game/Blueprints/g4.g4")
  (bind _asnote_block_bp_20 (Utilities|Casting|CastToNoteBlock_BP (Variables|/Script/Engine.ChildActorComponent|GetChildActor (Variables|Components|Geta4))))
  (Variables|/Game/Blueprints/NoteBlock_BP.NoteBlock_BP_C|SetNoteSound _asnote_block_bp_20 "/Game/Blueprints/a4.a4")
  (bind _asnote_block_bp_21 (Utilities|Casting|CastToNoteBlock_BP (Variables|/Script/Engine.ChildActorComponent|GetChildActor (Variables|Components|Getb4))))
  (Variables|/Game/Blueprints/NoteBlock_BP.NoteBlock_BP_C|SetNoteSound _asnote_block_bp_21 "/Game/Blueprints/b4.b4")
  (bind _asnote_block_bp_22 (Utilities|Casting|CastToNoteBlock_BP (Variables|/Script/Engine.ChildActorComponent|GetChildActor (Variables|Components|Getc5))))
  (Variables|/Game/Blueprints/NoteBlock_BP.NoteBlock_BP_C|SetNoteSound _asnote_block_bp_22 "/Game/Blueprints/c5.c5")
  (bind _asnote_block_bp_23 (Utilities|Casting|CastToNoteBlock_BP (Variables|/Script/Engine.ChildActorComponent|GetChildActor (Variables|Components|Getd5))))
  (Variables|/Game/Blueprints/NoteBlock_BP.NoteBlock_BP_C|SetNoteSound _asnote_block_bp_23 "/Game/Blueprints/d5.d5")
  (bind _asnote_block_bp_24 (Utilities|Casting|CastToNoteBlock_BP (Variables|/Script/Engine.ChildActorComponent|GetChildActor (Variables|Components|Gete5))))
  (Variables|/Game/Blueprints/NoteBlock_BP.NoteBlock_BP_C|SetNoteSound _asnote_block_bp_24 "/Game/Blueprints/e5.e5")
  (bind _asnote_block_bp_25 (Utilities|Casting|CastToNoteBlock_BP (Variables|/Script/Engine.ChildActorComponent|GetChildActor (Variables|Components|Getf5))))
  (Variables|/Game/Blueprints/NoteBlock_BP.NoteBlock_BP_C|SetNoteSound _asnote_block_bp_25 "/Game/Blueprints/f5.f5")
  (bind _asnote_block_bp_26 (Utilities|Casting|CastToNoteBlock_BP (Variables|/Script/Engine.ChildActorComponent|GetChildActor (Variables|Components|Getg5))))
  (Variables|/Game/Blueprints/NoteBlock_BP.NoteBlock_BP_C|SetNoteSound _asnote_block_bp_26 "/Game/Blueprints/g5.g5")
  (bind _asnote_block_bp_27 (Utilities|Casting|CastToNoteBlock_BP (Variables|/Script/Engine.ChildActorComponent|GetChildActor (Variables|Components|Getlolo))))
  (Variables|/Game/Blueprints/NoteBlock_BP.NoteBlock_BP_C|SetNoteSound _asnote_block_bp_27 "/Game/StarterContent/Audio/Explosion01.Explosion01")
  (bind _asnote_block_bp_28 (Utilities|Casting|CastToNoteBlock_BP (Variables|/Script/Engine.ChildActorComponent|GetChildActor (Variables|Components|Getlo))))
  (Variables|/Game/Blueprints/NoteBlock_BP.NoteBlock_BP_C|SetNoteSound _asnote_block_bp_28 "/Game/StarterContent/Audio/Explosion01.Explosion01")
  (bind _asnote_block_bp_29 (Utilities|Casting|CastToNoteBlock_BP (Variables|/Script/Engine.ChildActorComponent|GetChildActor (Variables|Components|Getfsharp2))))
  (Variables|/Game/Blueprints/NoteBlock_BP.NoteBlock_BP_C|SetNoteSound _asnote_block_bp_29 "/Game/Blueprints/f_2.f_2")
  (bind _asnote_block_bp_30 (Utilities|Casting|CastToNoteBlock_BP (Variables|/Script/Engine.ChildActorComponent|GetChildActor (Variables|Components|Getgsharp2))))
  (Variables|/Game/Blueprints/NoteBlock_BP.NoteBlock_BP_C|SetNoteSound _asnote_block_bp_30 "/Game/Blueprints/g_2.g_2")
  (bind _asnote_block_bp_31 (Utilities|Casting|CastToNoteBlock_BP (Variables|/Script/Engine.ChildActorComponent|GetChildActor (Variables|Components|Getasharp2))))
  (Variables|/Game/Blueprints/NoteBlock_BP.NoteBlock_BP_C|SetNoteSound _asnote_block_bp_31 "/Game/Blueprints/a_2.a_2")
  (bind _asnote_block_bp_32 (Utilities|Casting|CastToNoteBlock_BP (Variables|/Script/Engine.ChildActorComponent|GetChildActor (Variables|Components|Getcsharp3))))
  (Variables|/Game/Blueprints/NoteBlock_BP.NoteBlock_BP_C|SetNoteSound _asnote_block_bp_32 "/Game/Blueprints/c_3.c_3")
  (bind _asnote_block_bp_33 (Utilities|Casting|CastToNoteBlock_BP (Variables|/Script/Engine.ChildActorComponent|GetChildActor (Variables|Components|Getdsharp3))))
  (Variables|/Game/Blueprints/NoteBlock_BP.NoteBlock_BP_C|SetNoteSound _asnote_block_bp_33 "/Game/Blueprints/d_3.d_3")
  (bind _asnote_block_bp_34 (Utilities|Casting|CastToNoteBlock_BP (Variables|/Script/Engine.ChildActorComponent|GetChildActor (Variables|Components|Getfsharp3))))
  (Variables|/Game/Blueprints/NoteBlock_BP.NoteBlock_BP_C|SetNoteSound _asnote_block_bp_34 "/Game/Blueprints/f_3.f_3")
  (bind _asnote_block_bp_35 (Utilities|Casting|CastToNoteBlock_BP (Variables|/Script/Engine.ChildActorComponent|GetChildActor (Variables|Components|Getgsharp3))))
  (Variables|/Game/Blueprints/NoteBlock_BP.NoteBlock_BP_C|SetNoteSound _asnote_block_bp_35 "/Game/Blueprints/g_3.g_3")
  (bind _asnote_block_bp_36 (Utilities|Casting|CastToNoteBlock_BP (Variables|/Script/Engine.ChildActorComponent|GetChildActor (Variables|Components|Getasharp3))))
  (Variables|/Game/Blueprints/NoteBlock_BP.NoteBlock_BP_C|SetNoteSound _asnote_block_bp_36 "/Game/Blueprints/a_3.a_3")
  (bind _asnote_block_bp_37 (Utilities|Casting|CastToNoteBlock_BP (Variables|/Script/Engine.ChildActorComponent|GetChildActor (Variables|Components|Getcsharp4))))
  (Variables|/Game/Blueprints/NoteBlock_BP.NoteBlock_BP_C|SetNoteSound _asnote_block_bp_37 "/Game/Blueprints/c_4.c_4")
  (bind _asnote_block_bp_38 (Utilities|Casting|CastToNoteBlock_BP (Variables|/Script/Engine.ChildActorComponent|GetChildActor (Variables|Components|Getdsharp4))))
  (Variables|/Game/Blueprints/NoteBlock_BP.NoteBlock_BP_C|SetNoteSound _asnote_block_bp_38 "/Game/Blueprints/d_4.d_4")
  (bind _asnote_block_bp_39 (Utilities|Casting|CastToNoteBlock_BP (Variables|/Script/Engine.ChildActorComponent|GetChildActor (Variables|Components|Getfsharp4))))
  (Variables|/Game/Blueprints/NoteBlock_BP.NoteBlock_BP_C|SetNoteSound _asnote_block_bp_39 "/Game/Blueprints/f_4.f_4")
  (bind _asnote_block_bp_40 (Utilities|Casting|CastToNoteBlock_BP (Variables|/Script/Engine.ChildActorComponent|GetChildActor (Variables|Components|Getgsharp4))))
  (Variables|/Game/Blueprints/NoteBlock_BP.NoteBlock_BP_C|SetNoteSound _asnote_block_bp_40 "/Game/Blueprints/g_4.g_4")
  (bind _asnote_block_bp_41 (Utilities|Casting|CastToNoteBlock_BP (Variables|/Script/Engine.ChildActorComponent|GetChildActor (Variables|Components|Getasharp4))))
  (Variables|/Game/Blueprints/NoteBlock_BP.NoteBlock_BP_C|SetNoteSound _asnote_block_bp_41 "/Game/Blueprints/a_4.a_4")
  (bind _asnote_block_bp_42 (Utilities|Casting|CastToNoteBlock_BP (Variables|/Script/Engine.ChildActorComponent|GetChildActor (Variables|Components|Getcsharp5))))
  (Variables|/Game/Blueprints/NoteBlock_BP.NoteBlock_BP_C|SetNoteSound _asnote_block_bp_42 "/Game/Blueprints/c_5.c_5")
  (bind _asnote_block_bp_43 (Utilities|Casting|CastToNoteBlock_BP (Variables|/Script/Engine.ChildActorComponent|GetChildActor (Variables|Components|Getdsharp5))))
  (Variables|/Game/Blueprints/NoteBlock_BP.NoteBlock_BP_C|SetNoteSound _asnote_block_bp_43 "/Game/Blueprints/d_5.d_5")
  (bind _asnote_block_bp_44 (Utilities|Casting|CastToNoteBlock_BP (Variables|/Script/Engine.ChildActorComponent|GetChildActor (Variables|Components|Getfsharp5))))
  (Variables|/Game/Blueprints/NoteBlock_BP.NoteBlock_BP_C|SetNoteSound _asnote_block_bp_44 "/Game/Blueprints/f_5.f_5"))