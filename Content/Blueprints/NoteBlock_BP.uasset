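; NoteBlock_BP is a note block with a walnut-material cube that plays a sound when struck in VR or clicked.
; On overlap with either of the player pawn's motion controllers, it rumbles that controller and plays NoteSound in 2D.
; A mouse click plays the same sound without rumble.
; Despite its name, the playSound function only assigns a new NoteSound and does not play it.
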(event Collision|EventActorBeginOverlap
  (params (OtherActor :type Actor%20Object%20Reference))
  (bind _asmotion_controller_pawn (Utilities|Casting|CastToMotionControllerPawn (Game|Player|GetPlayerPawn 0)))
  (if (== OtherActor (Variables|/Game/VirtualRealityBP/Blueprints/MotionControllerPawn.MotionControllerPawn_C|GetLeftController _asmotion_controller_pawn))
    (Default|RumbleController (Variables|/Game/VirtualRealityBP/Blueprints/MotionControllerPawn.MotionControllerPawn_C|GetLeftController _asmotion_controller_pawn) 8.0)
    (Audio|PlaySound2D (Variables|Components|GetNoteSound) :!label _label)
    (elif (== OtherActor (Variables|/Game/VirtualRealityBP/Blueprints/MotionControllerPawn.MotionControllerPawn_C|GetRightController _asmotion_controller_pawn))
      (Default|RumbleController (Variables|/Game/VirtualRealityBP/Blueprints/MotionControllerPawn.MotionControllerPawn_C|GetRightController _asmotion_controller_pawn) 8.0)
      (goto _label))))

(event MouseInput|EventActorOnClicked
  (params (ButtonPressed :type Key%20Structure :default "AnyKey"))
  (Audio|PlaySound2D (Variables|Components|GetNoteSound)))

(fn ConstructionScript
  (Rendering|Material|SetMaterial (Variables|Default|GetCube) 0 "/Game/StarterContent/Materials/M_Wood_Walnut.M_Wood_Walnut")
  (Variables|Default|SetnotePlaying false))

(fn PlaySound
  (params (newSound :type Sound%20Wave%20Object%20Reference))
  (Variables|Components|SetNoteSound newSound))